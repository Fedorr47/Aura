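; Base Blueprint for item pickups, handling their spawn animation and spawn, ground impact and destruction sounds.
; On BeginPlay, a timeline drives scale and a height offset scaled by SpawnApex, firing the impact sound once when elevation dips below its start.
; When it finishes, rotation and sinusoidal movement start through functions defined outside this graph.
; Tick applies the calculated location and rotation; no overlap or collection logic is implemented here.
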(event EventBeginPlay
  (Audio|PlaySoundatLocation (Variables|Default|GetSpawnSound) (Transformation|GetActorLocation) "0, 0, 0" 1.0 1.0 0.0 0 0 0 0)
  (bind (_direction _newtrack_0 _newtrack_1) (Timeline|PickupElevation Play)
    (:Update
      (Variables|Default|SetElevation _newtrack_0)
      (Variables|Default|SetScale _newtrack_1)
      (Variables|Default|SetCalculatedLocation (CallFunction|CalculateElevation (Variables|Default|GetElevation)))
      (Transformation|SetActorScale3D (Math|Vector|MakeVector (Variables|Default|GetScale) (Variables|Default|GetScale) (Variables|Default|GetScale)))
      (if (< (Variables|Default|GetElevation) -0.1)
        (Utilities|FlowControl|DoOnce false
          (:Completed
            (Audio|PlaySoundatLocation (Variables|Default|GetGroundInpactSound) (Transformation|GetActorLocation) "0, 0, 0" 1.0 1.0 0.0 0 0 0 0)))))
    (:Finished
      (Class|AuraEffectActor|StartRotation)
      (Class|AuraEffectActor|StartSinusoidalMovement))))

(event Collision|EventActorBeginOverlap
  (params (OtherActor :type Actor%20Object%20Reference)))

(event EventTick
  (params (DeltaSeconds :type Float%20%28single-precision%29))
  (Transformation|SetActorLocation (Variables|Default|GetCalculatedLocation) false false)
  (Transformation|SetActorRotation (Variables|Default|GetCalculatedRotation)))

(event EventDestroyed
  (Audio|PlaySoundatLocation (Variables|Default|GetConsumedSound) (Transformation|GetActorLocation) "0, 0, 0" 1.0 1.0 0.0 0 0 0 0))

(fn ConstructionScript)

(fn CalculateElevation
  (params (Delta :type Float%20%28double-precision%29))
  (bind _initiallocation (Variables|Default|GetInitialLocation))
  (bind (_x _y _z) (Math|Vector|BreakVector _initiallocation))
  (return (Math|Vector|MakeVector _x _y (+ _z (* Delta (Variables|Default|GetSpawnApex))))))