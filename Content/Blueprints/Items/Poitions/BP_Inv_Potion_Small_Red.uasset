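; Small red potion item Blueprint that applies a gameplay effect to the player when the inventory signals a health effect.
; On BeginPlay it caches the inventory component from the first player controller and binds a handler to its health-effect delegate.
; The handler stores the received health amount and applies the configured gameplay effect class to the first player's pawn, without passing that amount into the call.
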(event Custom|CE_HealEffect
  (params (HealthAmount :type Float%20%28single-precision%29))
  (Variables|Default|SetHealth%20Amount HealthAmount)
  (Class|AuraEffectActor|ApplyEffecttoActor (Game|Player|GetPlayerPawn 0) (Variables|Default|GetInstantiateGameplayEffectClass)))

(event EventBeginPlay
  (bind _returnvalue (Class|InvInventoryStatics|GetInventoryComponent (Game|GetPlayerController 0)))
  (bind _output_get (Variables|Default|SetInventoryComponent _returnvalue))
  (Utilities|IsValid _output_get
    (:Is%20Valid
      (EventDispatchers|BindEventtoOnHealthEffectDelegate (Variables|Default|GetInventoryComponent) (delegate Custom|CE_HealEffect)))))

(event Collision|EventActorBeginOverlap
  (params (OtherActor :type Actor%20Object%20Reference)))

(event EventTick
  (params (DeltaSeconds :type Float%20%28single-precision%29)))

(fn ConstructionScript)