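; BP_Aura_MainMenu is the actor that sets up and animates the main menu scene.
; On BeginPlay it starts the menu music, adds WBP_MainMenu to the viewport and switches the player to UI-only input with a visible cursor.
; Each Tick bobs the fireball vertically around its starting position with an amplitude-scaled sine of accumulated time, reset past two pi.
; Tick also spins the magic circle decal at a frame-rate-independent rate.
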(event EventBeginPlay
  (Variables|Default|SetInitialFireballLocation (Transformation|GetWorldLocation (Variables|Default|GetFireBall)))
  (bind _returnvalue (Audio|SpawnSound2D "/Game/Assets/Sounds/Music/Music_MainMenu.Music_MainMenu" 1.0 1.0 0.0 0))
  (Variables|Default|SetMainMenuMusic _returnvalue)
  (bind _returnvalue_2 (UserInterface|CreateWidget "/Game/Blueprints/UI/MainMenu/WBP_MainMenu.WBP_MainMenu_C"))
  (bind _output_get (Variables|Default|SetMainMenuWidget _returnvalue_2))
  (Utilities|IsValid _output_get
    (:Is%20Valid
      (UserInterface|Viewport|AddtoViewport (Variables|Default|GetMainMenuWidget) 0)
      (Variables|Default|SetPlayerController (Game|GetPlayerController 0))
      (Input|SetInputModeUIOnly (Variables|Default|GetPlayerController) (Variables|Default|GetMainMenuWidget) "DoNotLock" false)
      (Variables|/Script/Engine.PlayerController|SetbShowMouseCursor (Variables|Default|GetPlayerController) true))))

(event Collision|EventActorBeginOverlap
  (params (OtherActor :type Actor%20Object%20Reference)))

(event EventTick
  (params (DeltaSeconds :type Float%20%28single-precision%29))
  (Transformation|SetWorldLocation (Variables|Default|GetFireBall) (+ (Variables|Default|GetInitialFireballLocation) (Math|Vector|MakeVector 0.0 0.0 (CallFunction|SineOfTime DeltaSeconds))) false false)
  (Transformation|AddLocalRotation (Variables|Default|GetMagicCircleDecal) (Math|Rotator|MakeRotator (* (Utilities|Time|GetWorldDeltaSeconds) (Variables|Default|GetMagicCircleRotationRate)) 0.0 0.0) false false))

(fn ConstructionScript)

(fn GetRadbyDeltaTime
  (params (Delta :type Float%20%28double-precision%29))
  (Variables|Default|SetTime (+ Delta (Variables|Default|GetTime)))
  (if (> (+ Delta (Variables|Default|GetTime)) (* (Math|Trig|GetPI) 2.0))
    (Variables|Default|SetTime 0.0))
  (return (Variables|Default|GetTime)))

(fn SineOfTime
  (params (DeltaTime :type Float%20%28double-precision%29))
  (return (* (Math|Trig|Sin(Radians) (CallFunction|GetRadbyDeltaTime DeltaTime)) (Variables|Default|GetAmplitude))))