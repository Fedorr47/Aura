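; BP_Goblin is a goblin enemy Blueprint with Spear and Slingshot variants selected by its Type variable.
; On BeginPlay it sets the matching weapon mesh, linked animation layer, hit-react montages, weapon dissolve material and character class (Warrior or Ranger).
; It then snaps the weapon to the WeaponHandleSocket on the body mesh.
; Tick, construction script and LinkAnimLayer are empty.
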(event EventBeginPlay
  (switch Utilities|FlowControl|Switch|SwitchonGoblinTypes (Variables|Default|GetType)
    (:Spear
      (Components|SkeletalMesh|SetSkeletalMeshAsset (Variables|Default|GetWeapon) "/Game/Assets/Enemies/Goblin/Spear/SKM_Spear.SKM_Spear")
      (Components|SkeletalMesh|AnimationBlueprintLinking|LinkAnimClassLayers (Variables|Character|GetMesh) "/Game/Blueprints/Enemies/AnimLogic/ABP_Goblin_Spear.ABP_Goblin_Spear_C")
      (Class|AuraCharacterBase|SetHitReactMontages (Variables|Default|GetIn%20Hit%20Montages%20Spear))
      (Variables|Default|SetWeaponDissolveMaterialInstance "/Game/Assets/Enemies/Goblin/Spear/Materials/MI_Spear_Dissolve.MI_Spear_Dissolve")
      (Variables|Default|SetCharacterClass "Warrior"))
    (:Slingshot
      (Components|SkeletalMesh|SetSkeletalMeshAsset (Variables|Default|GetWeapon) "/Game/Assets/Enemies/Goblin/Slingshot/Centered/SKM_Slingshot.SKM_Slingshot")
      (Components|SkeletalMesh|AnimationBlueprintLinking|LinkAnimClassLayers (Variables|Character|GetMesh) "/Game/Blueprints/Enemies/AnimLogic/ABP_Goblin_SlingShot.ABP_Goblin_SlingShot_C")
      (Class|AuraCharacterBase|SetHitReactMontages (Variables|Default|GetIn%20Hit%20Montages%20SlingShot))
      (Variables|Default|SetWeaponDissolveMaterialInstance "/Game/Assets/Enemies/Goblin/Slingshot/Materials/Red/MI_Slingshot_Red_Dissolve.MI_Slingshot_Red_Dissolve")
      (Variables|Default|SetCharacterClass "Ranger")))
  (Transformation|AttachComponentToComponent (Variables|Default|GetWeapon) (Variables|Character|GetMesh) "WeaponHandleSocket" "SnapToTarget" "SnapToTarget" "SnapToTarget" true))

(event Collision|EventActorBeginOverlap
  (params (OtherActor :type Actor%20Object%20Reference)))

(event EventTick
  (params (DeltaSeconds :type Float%20%28single-precision%29)))

(fn ConstructionScript)

(fn LinkAnimLayer)