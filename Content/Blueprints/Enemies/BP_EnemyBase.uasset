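; BP_EnemyBase is an enemy base Blueprint that handles spawn scale-in, dissolve effects, facing and loot drops.
; Timelines drive the mesh scale on BeginPlay and the Dissolve parameter on body and weapon materials, while motion warping updates a FacingTarget.
; SpawnLoot rolls loot tiers, then a looping timer spawns items one by one in an evenly spaced ring at random distances.
; AuraEffectActor loot inherits the enemy's level; the level-override branch is empty.
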(event Custom|SpawnLootItems
  (bind _spawnloopcount (Variables|Default|GetSpawnLoopCount))
  (bind _lootitems (Variables|Default|GetLootItems))
  (bind _output (Utilities|Array|Get(acopy) _lootitems _spawnloopcount))
  (bind (_lootclass _bloottleveloverride) (Utilities|Struct|BreakLootItem _output))
  (if (< (Variables|Default|GetSpawnLoopCount) (Utilities|Array|Length (Variables|Default|GetLootItems)))
    (Variables|Default|SetLoot%20Class _lootclass)
    (Variables|Default|SetLoott%20Level%20Override _bloottleveloverride)
    (bind _returnvalue (Game|SpawnActorfromClass (Variables|Default|GetLoot%20Class) (CallFunction|GetLootTransform (Variables|Default|GetSpawnLoopCount)) "AdjustIfPossibleButDontSpawnIfColliding" "MultiplyWithRoot" 0 0))
    (bind _asaura_effect_actor (Utilities|Casting|CastToAuraEffectActor _returnvalue)
      (:then
        (Variables|/Script/Aura.AuraEffectActor|SetActorLevel _asaura_effect_actor (Math|Conversions|ToFloat(Integer) (Variables|Default|GetLevel))))
      (:CastFailed
        _))
    (if (Variables|Default|GetLoott%20Level%20Override)
      _
      (else
        _))
    (Math|Integer|IncrementInt (Variables|Default|GetSpawnLoopCount))
    (else
      (Utilities|Time|ClearandInvalidateTimerbyHandle (Variables|Default|GetLootTimer)))))

(event EventBeginPlay
  (bind _spawntime (Timeline|Spawn%20timeline Play)
    (:Update
      (Transformation|SetRelativeScale3D (Variables|Character|GetMesh) (Math|Vector|MakeVector _spawntime _spawntime _spawntime)))))

(event Collision|EventActorBeginOverlap
  (params (OtherActor :type Actor%20Object%20Reference)))

(event EventTick
  (params (DeltaSeconds :type Float%20%28single-precision%29)))

(event EventStartDissolveTimeLine
  (params (DynamicMaterialInstance :type Material%20Instance%20Dynamic%20Object%20Reference))
  (bind _dissolve (Timeline|Dissolve Play)
    (:Update
      (Rendering|Material|SetScalarParameterValue DynamicMaterialInstance "Dissolve" _dissolve :!class /Script/Engine.MaterialInstanceDynamic))))

(event EventStartWeaponDissolveTimeLine
  (params (DynamicMaterialInstance :type Material%20Instance%20Dynamic%20Object%20Reference))
  (bind _dissolve (Timeline|WeaponDissolve Play)
    (:Update
      (Rendering|Material|SetScalarParameterValue DynamicMaterialInstance "Dissolve" _dissolve :!class /Script/Engine.MaterialInstanceDynamic))))

(event EventSetFacingWrapping
  (params (TargetLocation :type Vector%20%28by%20ref%29 :default "0, 0, 0"))
  (Class|MotionWarpingComponent|AddorUpdateWarpTargetfromLocation (Variables|Default|GetMotionWarping) "FacingTarget" TargetLocation))

(event EventSpawnLoot
  (bind _returnvalue (Class|AuraAbilitySystemLibrary|GetLootTiers))
  (Utilities|IsValid _returnvalue
    (:Is%20Valid
      (bind _returnvalue_2 (Class|LootTiers|GetLootItems _returnvalue))
      (bind _output_get (Variables|Default|SetLootItems _returnvalue_2))
      (Variables|Default|SetLootRotations (CallFunction|GetLootRotations _output_get))
      (bind _returnvalue_3 (Utilities|Time|SetTimerbyEvent (delegate Custom|SpawnLootItems) 0.1 true))
      (Variables|Default|SetLootTimer _returnvalue_3)
      (CallFunction|SpawnLootItems))))

(fn ConstructionScript)

(fn GetLootRotations
  (params (LootIteems :type Array%20of%20Loot%20Item%20Structures))
  (return (Class|AuraAbilitySystemLibrary|EvenlySpaceRotators (Transformation|GetActorForwardVector) (Math|Vector|VectorUp) 3.6e+02 (Utilities|Array|Length LootIteems))))

(fn GetLootTransform
  (params (LootCount :type Integer))
  (bind _lootrotations (Variables|Default|GetLootRotations))
  (bind _output (Utilities|Array|Get(acopy) _lootrotations LootCount))
  (return (Math|Transform|MakeTransform (+ (* (Math|Vector|GetForwardVector _output) (Math|Random|RandomFloatinRange (Variables|Default|GetMinSpawnDistnace) (Variables|Default|GetMaxSpawnDistnace))) (Transformation|GetActorLocation)) _output)))