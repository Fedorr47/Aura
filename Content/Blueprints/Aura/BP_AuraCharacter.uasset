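; Player character Blueprint for Aura that links the staff animation layers to its mesh on BeginPlay.
; Events update a motion warping target for facing a location and store the attack loop state.
; A box overlap sends fade out and fade in messages to actors implementing BPI_FadeInterface as they enter and leave.
; The debug key leads to an empty FlipFlop, and the overhead name and input mode logic never runs.
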(event OnComponentBeginOverlap(Box)
  (params (OverlappedComponent :type Primitive%20Component%20Object%20Reference) (OtherActor :type Actor%20Object%20Reference) (OtherComp :type Primitive%20Component%20Object%20Reference) (OtherBodyIndex :type Integer) (bFromSweep :type Boolean) (SweepResult :type Hit%20Result%20Structure%20%28by%20ref%29))
  (if (Utilities|DoesObjectImplementInterface OtherActor "/Game/Blueprints/Interfaces/BPI_FadeInterface.BPI_FadeInterface_C")
    (Class|BPIFadeInterface|FadeOut(Message) OtherActor)))

(event OnComponentEndOverlap(Box)
  (params (OverlappedComponent :type Primitive%20Component%20Object%20Reference) (OtherActor :type Actor%20Object%20Reference) (OtherComp :type Primitive%20Component%20Object%20Reference) (OtherBodyIndex :type Integer))
  (if (Utilities|DoesObjectImplementInterface OtherActor "/Game/Blueprints/Interfaces/BPI_FadeInterface.BPI_FadeInterface_C")
    (Class|BPIFadeInterface|Fadein(Message) OtherActor)))

(event EventBeginPlay
  (Components|SkeletalMesh|AnimationBlueprintLinking|LinkAnimClassLayers (Variables|Character|GetMesh) "/Game/Blueprints/Aura/AnimLogic/Aura/ABP_Staff.ABP_Staff_C"))

(event Collision|EventActorBeginOverlap
  (params (OtherActor :type Actor%20Object%20Reference)))

(event EventTick
  (params (DeltaSeconds :type Float%20%28single-precision%29)))

(event EventSetinAttackLoop
  (params (InLoop :type Boolean))
  (Variables|AuraCharacter|SetInAttackLoop InLoop))

(event EventSetFacingWarping
  (params (TargetLocation :type Vector%20%28by%20ref%29 :default "0, 0, 0"))
  (Class|MotionWarpingComponent|AddorUpdateWarpTargetfromLocation (Variables|Default|GetMotionWarping) "FacingTarget" TargetLocation))

(event Input|KeyboardEvents|DebugKeyC
  (params (Key :type Key%20Structure :default "None") (ActionValue :type Input%20Action%20Value%20Structure))
  (:Pressed
    (Utilities|FlowControl|FlipFlop)))

(fn ConstructionScript)