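; Arcane Shards gameplay ability: erupts a series of damaging shards around a cursor-targeted ground point, their count scaling with level up to a cap.
; It shows a magic circle until confirmed input, then spawns a temporary point collection for randomly rotated ground locations and plays the cast montage.
; The montage event starts a looping timer that, per point, deals radial damage with outward knockback and fires a GameplayCue, then ends the ability.
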(event Custom|EventSpawmShard
  (if (< (Variables|Default|GetCurrentIndexOfPoint) (Variables|Default|GetNum%20Points))
    (CallFunction|StoreShardSpawnLocation)
    (CallFunction|GetPawntoDamage)
    (for _array_element (Variables|Default|GetPawnsToDamage)
      (CallFunction|DoRadialDamage _array_element))
    (Math|Integer|IncrementInt (Variables|Default|GetCurrentIndexOfPoint)
      (:%20%20
        (Class|GameplayAbility|ExecuteGameplayCuewithParams "(TagName=\"GameplayCue.ArcaneShards\")" (Ability|GameplayCue|MakeGameplayCueParameters :Location (Variables|Default|GetShardSpawnLocation)))))
    (else
      (Utilities|Time|ClearandInvalidateTimerbyHandle (Variables|Default|GetShardTimer))
      (Actor|DestroyActor (Variables|Default|GetPointCollection))
      (Ability|EndAbility))))

(event Ability|EventActivateAbility
  (bind _returnvalue (Class|GameplayAbility|CheckAbilityCost))
  (if _returnvalue
    (Variables|Default|SetCurrentIndexOfPoint 0)
    (Variables|Default|SetNum%20Points (Math|Integer|Min(Integer) (Ability|GetAbilityLevel) (Variables|Default|GetMaxShardPoints)))
    (Utilities|FlowControl|Sequence
      (:then_0
        (Class|PlayerInterface|ShowMagicCircle(Message) (Ability|GetAvatarActorfromActorInfo)))
      (:then_1
        (Ability|Tasks|WaitInputPress false
          (:OnPress
            (bind _datahandle (|TargetDataUnderCursor)
              (:ValidData
                (Ability|CommitAbilityCost false)
                (Variables|Default|SetMouseHitLocation (.ImpactPoint (Collision|BreakHitResult (Ability|TargetData|GetHitResultfromTargetData _datahandle))))
                (Utilities|FlowControl|Sequence
                  (:then_0
                    (bind _returnvalue_2 (Game|SpawnActorfromClass "/Game/Blueprints/AbilitySystem/Aura/Abilities/Arcane/ArcaneShards/BP_PointCollection.BP_PointCollection_C" (Math|Transform|MakeTransform (Variables|Default|GetMouseHitLocation) "0, 0, 0" "1.000000,1.000000,1.000000") "AlwaysSpawn" "MultiplyWithRoot" 0 0))
                    (bind _output_get (Variables|Default|SetPointCollection _returnvalue_2))
                    (Variables|Default|SetCashedValue (Class|PointCollection|GetGroundPoints _output_get (Variables|Default|GetMouseHitLocation) (Variables|Default|GetNum%20Points) (Math|Random|RandomFloatinRange 0.0 3.6e+02))))
                  (:then_1
                    (Class|CombatInterface|SetFacingWarping(Message) (Ability|GetAvatarActorfromActorInfo) (Variables|Default|GetMouseHitLocation)))
                  (:then_2
                    (|PlayMontageandWaitProxy "None" "/Game/Blueprints/Thorne/AM_Cast_ArcaneShards_Short.AM_Cast_ArcaneShards_Short" 1.0 "None" false 1.0 0.0 false
                      (:then
                        (Ability|Tasks|WaitGameplayEvent "(TagName=\"Event.Montage.ArcaneShards\")" 0 true
                          (:then
                            (bind _returnvalue_3 (Utilities|Time|SetTimerbyEvent (delegate Custom|EventSpawmShard) (Variables|Default|GetShardSpawmDeltaTime) true true))
                            (Variables|Default|SetShardTimer _returnvalue_3)
                            (Class|PlayerInterface|HideMagicCircle(Message) (Ability|GetAvatarActorfromActorInfo))
                            (CallFunction|EventSpawmShard)
                            (Ability|CommitAbilityCooldown false)))))))))))))))

(event Ability|EventOnEndAbility
  (params (bWasCancelled :type Boolean)))

(fn StoreShardSpawnLocation
  (Variables|Default|SetShardSpawnLocation (Transformation|GetWorldLocation (Utilities|Array|Get(acopy) (Variables|Default|GetCashedValue) (Variables|Default|GetCurrentIndexOfPoint)))))

(fn GetPawntoDamage
  (bind _returnvalue (Ability|GetAvatarActorfromActorInfo))
  (bind _outoverlappingactors (Class|AuraAbilitySystemLibrary|GetLivePlayerswithRadius _returnvalue (Utilities|Array|MakeArray _returnvalue) (Variables|Default|GetRadialDamageOuterRadius) (Variables|Default|GetShardSpawnLocation)))
  (Variables|Default|SetPawnsToDamage _outoverlappingactors))

(fn DoRadialDamage
  (params (TargetActor :type Actor%20Object%20Reference))
  (bind _returnvalue (Transformation|GetActorLocation TargetActor))
  (bind _shardspawnlocation (Variables|Default|GetShardSpawnLocation))
  (bind _returnvalue_2 (- _returnvalue _shardspawnlocation))
  (Class|AuraAbilitySystemLibrary|DoDamage (Class|AuraDamageGameplayAbility|MakeDamageEffectParamsfromDefaultClass TargetActor (Variables|Default|GetShardSpawnLocation) true _returnvalue_2 true _returnvalue_2 true 35.0)))