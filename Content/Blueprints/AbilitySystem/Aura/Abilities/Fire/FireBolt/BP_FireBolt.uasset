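; BP_FireBolt is the Fire Bolt ability's actor, which destroys itself when it stops moving.
; On BeginPlay it waits briefly, then sets the Sphere component's collision to query-only.
; Each tick it compares its current and previous locations and destroys itself if the distance travelled is at or below MinDistanceOverFrame.
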(event EventBeginPlay
  (Utilities|FlowControl|Delay 0.05)
  (bind _sphere (Variables|Default|GetSphere)
    (:then
      (Collision|SetCollisionEnabled _sphere "QueryOnly"))
    (:else)))

(event Collision|EventActorBeginOverlap
  (params (OtherActor :type Actor%20Object%20Reference)))

(event EventTick
  (params (DeltaSeconds :type Float%20%28single-precision%29))
  (Variables|Default|SetLastFrameLocation (Variables|Default|GetThisFrameLocation))
  (Variables|Default|SetThisFrameLocation (Transformation|GetActorLocation))
  (if (<= (Math|Vector|VectorLength (- (Variables|Default|GetLastFrameLocation) (Variables|Default|GetThisFrameLocation))) (Variables|Default|GetMinDistanceOverFrame))
    (Actor|DestroyActor)))

(fn ConstructionScript)