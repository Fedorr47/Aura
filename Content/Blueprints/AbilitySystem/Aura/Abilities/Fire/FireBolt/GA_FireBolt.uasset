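; GA_FireBolt is the mage's Fire Bolt gameplay ability, which launches projectiles at the target under the cursor.
; On activation it commits, stores the hit location and actor from cursor target data, warps the avatar's facing and plays the cast montage.
; A montage gameplay event triggers SpawnProjectiles with a pitch override and the hit actor as homing target.
; The ability ends when the montage completes, blends out, is interrupted or is cancelled.
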(event Ability|EventActivateAbility
  (Ability|CommitAbility)
  (bind _datahandle (|TargetDataUnderCursor)
    (:ValidData
      (Variables|Default|SetProjectileTargetLocation (.Location (Collision|BreakHitResult (Ability|TargetData|GetHitResultfromTargetData _datahandle))))
      (Variables|Default|SetMouseHitActor (.HitActor (Collision|BreakHitResult (Ability|TargetData|GetHitResultfromTargetData _datahandle))))
      (Class|CombatInterface|SetFacingWarping(Message) (Ability|GetAvatarActorfromActorInfo) (Variables|Default|GetProjectileTargetLocation))
      (|PlayMontageandWaitProxy "None" "/Game/Blueprints/Mage/Animations/AM_Mage_Сast_FireBolt.AM_Mage_Сast_FireBolt" 1.0 "None" false 1.0 0.0 false
        (:then
          (Ability|Tasks|WaitGameplayEvent "(TagName=\"Event.Montage.FireBolt\")" 0 true
            (:EventReceived
              (Class|AuraFireBolt|SpawnProjectiles (Variables|Default|GetProjectileTargetLocation) (Variables|Default|GetSocket%20Type) true (Variables|Default|GetMouseHitActor) 2e+01))))
        (:OnCompleted
          (Ability|EndAbility :!label _label))
        (:OnBlendOut
          (goto _label))
        (:OnInterrupted
          (goto _label))
        (:OnCancelled
          (goto _label))))))

(event Ability|EventOnEndAbility
  (params (bWasCancelled :type Boolean)))