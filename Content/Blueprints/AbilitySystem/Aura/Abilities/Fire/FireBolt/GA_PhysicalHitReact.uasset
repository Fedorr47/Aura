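; Gameplay ability that makes its avatar play a physical hit reaction.
; On activation it applies the hit reaction gameplay effect to the owner, then plays the montage the avatar's CombatInterface returns for the hit react type.
; When the montage completes, is interrupted or is cancelled, it removes the effect by its stored handle and ends.
; If the interface cast fails, the effect stays applied and the ability never calls EndAbility.
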(event Ability|EventActivateAbility
  (bind _returnvalue (Ability|ApplyGameplayEffectToOwner (Variables|Default|GetHitReactionEffectClass)))
  (Variables|Default|SetHitReactionEffect _returnvalue)
  (bind _ascombat_interface (Utilities|Casting|CastToCombatInterface (Ability|GetAvatarActorfromActorInfo)))
  (bind _output_get (Variables|Default|SetCommbatActor _ascombat_interface))
  (bind _returnvalue_2 (Class|CombatInterface|GetHitReactMontage _output_get (Variables|Default|GetHitReactType)))
  (|PlayMontageandWaitProxy "None" _returnvalue_2 1.0 "None" true 1.0 0.0 false
    (:OnCompleted
      _)
    (:OnInterrupted
      _)
    (:OnCancelled
      _))
  (Ability|RemoveGameplayEffectFromOwnerWithHandle (Variables|Default|GetHitReactionEffect))
  (Ability|EndAbility))

(event Ability|EventOnEndAbility
  (params (bWasCancelled :type Boolean)))