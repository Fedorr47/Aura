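; Fireball actor for the Aura FireBlast ability that flies outward, returns to its caster and explodes on arrival.
; On the server, two chained timelines lerp it forward by TravelDistance, then back toward the caster's current location.
; Within ExplodeDistance of the caster, it calls OnHit, applies radial damage with knockback and death impulses to nearby live players except the caster, then destroys itself.
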(event EventStartOutgoingTimeline
  (Networking|SwitchHasAuthority
    (:Authority
      (Variables|Default|SetCaster (Game|GetInstigator))
      (Variables|Default|SetCurrentPosition (Transformation|GetActorLocation))
      (Variables|Default|SetReturnPosition (+ (Variables|Default|GetCurrentPosition) (* (Transformation|GetActorForwardVector) (Variables|Default|GetTravelDistance))))
      (bind _fromcaster (Timeline|FromCaster Play)
        (:Update
          (Transformation|SetActorLocation (Math|Vector|Lerp(Vector) (Variables|Default|GetCurrentPosition) (Variables|Default|GetReturnPosition) _fromcaster) false false))
        (:Finished
          (bind _tocaster (Timeline|ToCaster Play)
            (:Update
              (Transformation|SetActorLocation (Math|Vector|Lerp(Vector) (Variables|Default|GetReturnPosition) (Transformation|GetActorLocation (Variables|Default|GetCaster)) _tocaster) false false)
              (if (CallFunction|OnExplosionDistance)
                (Class|AuraProjectile|OnHit)
                (Class|AuraAbilitySystemLibrary|SetIsRadialDamageEffectParam (Variables|Default|GetExplosionDamageParams) true 5e+01 2e+02 (Transformation|GetActorLocation))
                (Utilities|Array|Add (Utilities|Array|MakeArray (Variables|Default|GetCaster)) self)
                (bind _outoverlappingactors (Class|AuraAbilitySystemLibrary|GetLivePlayerswithRadius self (Utilities|Array|MakeArray (Variables|Default|GetCaster)) 3e+02 (Transformation|GetActorLocation)))
                (bind _output_get (Variables|Default|SetOut%20Overlapping%20Actors _outoverlappingactors))
                (for _array_element _output_get
                  (Class|AuraAbilitySystemLibrary|SetTargetASCDamageEffectParam (Variables|Default|GetExplosionDamageParams) (Ability|GetAbilitySystemComponent _array_element))
                  (Variables|Default|SetImpulseDirection (- (Transformation|GetActorLocation _array_element) (Transformation|GetActorLocation)))
                  (Class|AuraAbilitySystemLibrary|SetKnockBackImpulseDamageEffectParam (Variables|Default|GetExplosionDamageParams) (CallFunction|PitchOverrideImpulse) 8e+02)
                  (Class|AuraAbilitySystemLibrary|SetDeathImpulseDamageEffectParam (Variables|Default|GetExplosionDamageParams) (Variables|Default|GetImpulseDirection) 6e+02)
                  (Class|AuraAbilitySystemLibrary|DoDamage (Variables|Default|GetExplosionDamageParams)))
                (Actor|DestroyActor)))
            (:Finished
              (Actor|DestroyActor))))))))

(fn ConstructionScript)

(fn OnExplosionDistance
  (return (<= (Math|Vector|VectorLength (- (Transformation|GetActorLocation) (Transformation|GetActorLocation (Variables|Default|GetCaster)))) (Variables|Default|GetExplodeDistance))))

(fn PitchOverrideImpulse
  (bind _impulsedirection (Variables|Default|GetImpulseDirection))
  (bind _returnvalue (Math|Rotator|MakeRotfromX _impulsedirection))
  (return (Math|Vector|MakeVector (.roll _returnvalue) 45.0 (.yaw _returnvalue))))