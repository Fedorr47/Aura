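; Electrocute gameplay ability: a channeled lightning beam cast at the cursor target that chains to additional targets.
; A montage event locks movement, adds shock-loop gameplay cues and starts a looping timer that commits cost and applies set-by-caller lightning damage.
; Input release (with server-delayed minimum hold), failed cost or primary target death ends it, restoring movement, removing cues and committing cooldown.
; Ending also deals final server-side damage to combat targets.
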(event Custom|EventDamageAndCost
  (bind _returnvalue (Ability|CommitAbilityCost false))
  (if _returnvalue
    (CallFunction|ApplyDamage)
    (else
      (CallFunction|ClearTimerandEndAbility))))

(event Ability|EventActivateAbility
  (CallFunction|ChecktoCombatInterface)
  (bind _datahandle (|TargetDataUnderCursor)
    (:ValidData
      (Class|AuraBeamSpell|StoreMouseDataInfo (Ability|TargetData|GetHitResultfromTargetData _datahandle))
      (Class|AuraBeamSpell|StoreOwnerVariables)
      (Utilities|FlowControl|Sequence
        (:then_0
          (bind _ownerplayercontroller (Variables|Default|GetOwnerPlayerController)
            (:then
              (Variables|/Script/Engine.PlayerController|SetbShowMouseCursor _ownerplayercontroller false)
              (CallFunction|SetFacingTarget)
              (GameplayCue|ExecuteGameplayCue :GameplayCueTag "(TagName=\"GameplayCue.ShockBurst\")")
              (|PlayMontageandWaitProxy "None" (Variables|Default|GetMontageElectrocute) 1.0 "None" false 1.0 0.0 false
                (:then
                  (Ability|Tasks|WaitGameplayEvent "(TagName=\"Event.Montage.Electrocute\")" 0 true
                    (:EventReceived
                      (CallFunction|InShockLoop)
                      (CallFunction|SpawnElectoBeam)
                      (bind _returnvalue (Utilities|Time|SetTimerbyEvent (delegate Custom|EventDamageAndCost) (Variables|Default|GetDamageDeltaTime) true))
                      (Variables|Default|SetDamageAndCostTimer _returnvalue))))))
            (:else)))
        (:then_1
          (bind _timeheld (Ability|Tasks|WaitInputRelease false)
            (:OnRelease
              (Variables|Default|SetTime%20Held _timeheld)
              (if (< (Variables|Default|GetTime%20Held) (Variables|Default|GetMinSpellTime))
                (Ability|HasAuthority
                  (:True
                    (Utilities|FlowControl|Delay (- (Variables|Default|GetMinSpellTime) (Variables|Default|GetTime%20Held)))
                    (CallFunction|ClearTimerandEndAbility :!label _label))
                  (:False
                    (CallFunction|PreparetoEndAbility)))
                (else
                  (goto _label))))))))))

(event Ability|EventOnEndAbility
  (params (bWasCancelled :type Boolean)))

(event EventPrimaryTargetDied
  (params (DiedActor :type Actor%20Object%20Reference))
  (GameplayCue|RemoveGameplayCueOnActor(Looping) DiedActor "(TagName=\"GameplayCue.ShookLoop\")" (Variables|Default|GetFirstTargetCueParameters))
  (CallFunction|ClearTimerandEndAbility))

(event EventAdditionalTargetDied
  (params (DiedActor :type Actor%20Object%20Reference))
  (CallFunction|RemoveShockLoopfromAdditionalTarget DiedActor)
  (Utilities|Array|RemoveItem (Variables|Default|GetAdditionalTargets) DiedActor))

(fn ChecktoCombatInterface
  (if (Utilities|DoesObjectImplementInterface (Ability|GetAvatarActorfromActorInfo) "/Script/Aura.CombatInterface")
    (return)
    (else
      (Ability|EndAbility))))

(fn PreparetoEndAbility
  (Variables|/Script/Engine.PlayerController|SetbShowMouseCursor (Variables|Default|GetOwnerPlayerController) true)
  (Class|CombatInterface|SetinAttackLoop(Message) (Ability|GetAvatarActorfromActorInfo) false)
  (Pawn|Components|CharacterMovement|SetMovementMode (Variables|/Script/Engine.Character|GetCharacterMovement (Variables|Default|GetOwnerCharacter)) "MOVE_Walking" 0)
  (if (Variables|Default|GetIsCombatActor)
    (Class|CombatInterface|SetBeinginShock(Message) (Variables|Default|GetMouseHitActor) false)
    (GameplayCue|RemoveGameplayCueOnActor(Looping) (Variables|Default|GetMouseHitActor) "(TagName=\"GameplayCue.ShookLoop\")" (Variables|Default|GetFirstTargetCueParameters))
    (Ability|HasAuthority
      (:True
        (Class|AuraAbilitySystemLibrary|DoDamage (Class|AuraDamageGameplayAbility|MakeDamageEffectParamsfromDefaultClass (Variables|Default|GetMouseHitActor) "0, 0, 0" false "0, 0, 0" false "0, 0, 0" false 0.0)))
      (:False
        _))
    (for _array_element (Variables|Default|GetAdditionalTargets)
      (Class|CombatInterface|SetBeinginShock(Message) _array_element false)
      (CallFunction|RemoveShockLoopfromAdditionalTarget _array_element)
      (Ability|HasAuthority
        (:True
          (Class|AuraAbilitySystemLibrary|DoDamage (Class|AuraDamageGameplayAbility|MakeDamageEffectParamsfromDefaultClass _array_element "0, 0, 0" false "0, 0, 0" false "0, 0, 0" false 0.0)))))
    (else
      (GameplayCue|RemoveGameplayCueOnActor(Looping) (Ability|GetAvatarActorfromActorInfo) "(TagName=\"GameplayCue.ShookLoop\")" (Variables|Default|GetFirstTargetCueParameters)))))

(fn InShockLoop
  (Class|CombatInterface|SetinAttackLoop(Message) (Ability|GetAvatarActorfromActorInfo) true)
  (Pawn|Components|CharacterMovement|DisableMovement (Variables|/Script/Engine.Character|GetCharacterMovement (Variables|Default|GetOwnerCharacter))))

(fn SetFacingTarget
  (Class|CombatInterface|SetFacingWarping(Message) (Ability|GetAvatarActorfromActorInfo) (Variables|Default|GetMouseHitLocation)))

(fn SpawnElectoBeam
  (Class|AuraBeamSpell|TraceFirstTarget (Variables|Default|GetMouseHitLocation))
  (bind _returnvalue (Class|CombatInterface|GetWeapon(Message) (Variables|Default|GetOwnerCharacter)))
  (LocalVariables|SetWeapon _returnvalue)
  (Variables|Default|SetFirstTargetCueParameters (Ability|GameplayCue|MakeGameplayCueParameters :Location (Variables|Default|GetMouseHitLocation) :SourceObject (Variables|Default|GetMouseHitActor) :TargetAttachComponent (LocalVariables|GetWeapon)))
  (bind _output_get (Variables|Default|SetIsCombatActor (Utilities|DoesObjectImplementInterface (Variables|Default|GetMouseHitActor) "/Script/Aura.CombatInterface")))
  (if _output_get
    (LocalVariables|SetCueTarget (Variables|Default|GetMouseHitActor))
    (else
      (LocalVariables|SetCueTarget (Ability|GetAvatarActorfromActorInfo))))
  (GameplayCue|AddGameplayCueOnActor(Looping) (LocalVariables|GetCueTarget) "(TagName=\"GameplayCue.ShookLoop\")" (Variables|Default|GetFirstTargetCueParameters))
  (if (Variables|Default|GetIsCombatActor)
    (Class|CombatInterface|SetBeinginShock(Message) (LocalVariables|GetCueTarget) true)
    (bind _outadditionaltargets (Class|AuraBeamSpell|StoreAdditionalTargets))
    (bind _output_get_2 (Variables|Default|SetAdditionalTargets _outadditionaltargets))
    (for _array_element _output_get_2
      (Class|CombatInterface|SetBeinginShock(Message) _array_element true)
      (CallFunction|AddShockLoopCuetoActor _array_element))))

(fn AddShockLoopCuetoActor
  (params (TargetActor :type Actor%20Object%20Reference))
  (LocalVariables|SetActorTarget TargetActor)
  (Utilities|Map|Add (Variables|Default|GetAdditionalActorsToCueParams) (LocalVariables|GetActorTarget) (Ability|GameplayCue|MakeGameplayCueParameters :Location (Transformation|GetActorLocation (LocalVariables|GetActorTarget)) :SourceObject (LocalVariables|GetActorTarget) :TargetAttachComponent (Variables|/Script/Engine.Actor|GetRootComponent (Variables|Default|GetMouseHitActor))))
  (GameplayCue|AddGameplayCueOnActor(Looping) (LocalVariables|GetActorTarget) "(TagName=\"GameplayCue.ShookLoop\")" (Ability|GameplayCue|MakeGameplayCueParameters :Location (Transformation|GetActorLocation (LocalVariables|GetActorTarget)) :SourceObject (LocalVariables|GetActorTarget) :TargetAttachComponent (Variables|/Script/Engine.Actor|GetRootComponent (Variables|Default|GetMouseHitActor)))))

(fn RemoveShockLoopfromAdditionalTarget
  (params (AdditionalTarget :type Actor%20Object%20Reference))
  (bind _additionalactorstocueparams (Variables|Default|GetAdditionalActorsToCueParams))
  (bind (_value _returnvalue) (Utilities|Map|Find _additionalactorstocueparams AdditionalTarget))
  (if _returnvalue
    (GameplayCue|RemoveGameplayCueOnActor(Looping) AdditionalTarget "(TagName=\"GameplayCue.ShookLoop\")" _value)))

(fn ApplyDamage
  (CallFunction|ApplyDamageSingleTarget (Variables|Default|GetMouseHitActor))
  (for _array_element (Variables|Default|GetAdditionalTargets)
    (CallFunction|ApplyDamageSingleTarget _array_element)))

(fn ApplyDamageSingleTarget
  (params (HitActor :type Actor%20Object%20Reference))
  (bind _returnvalue (Ability|GetAbilitySystemComponent HitActor))
  (Utilities|IsValid HitActor
    (:Is%20Valid
      (bind _output_get (LocalVariables|SetASC (Ability|GetAbilitySystemComponentfromActorInfo)))
      (Utilities|IsValid _output_get
        (:Is%20Valid
          (bind _returnvalue_2 (Ability|GameplayEffect|AssignTagSetbyCallerMagnitude (GameplayEffects|MakeOutgoingSpec (LocalVariables|GetASC) (Variables|Default|GetDamageEffectClass) (Math|Conversions|ToFloat(Integer) (Ability|GetAbilityLevel)) (GameplayEffects|MakeEffectContext (LocalVariables|GetASC))) "(TagName=\"Damage.Lightning\")" (Class|AuraDamageGameplayAbility|GetDamageatLevel)))
          (Utilities|IsValid _returnvalue
            (:Is%20Valid
              (GameplayEffects|ApplyGameplayEffectSpecToSelf _returnvalue _returnvalue_2))))))))

(fn ClearTimerandEndAbility
  (Utilities|Time|ClearandInvalidateTimerbyHandle (Variables|Default|GetDamageAndCostTimer))
  (CallFunction|PreparetoEndAbility)
  (Ability|CommitAbilityCooldown false)
  (Utilities|Array|Clear (Variables|Default|GetAdditionalTargets))
  (Utilities|Map|Clear (Variables|Default|GetAdditionalActorsToCueParams))
  (Variables|Default|SetMouseHitActor 0)
  (Variables|Default|SetIsCombatActor false)
  (Variables|Default|SetTime%20Held 0.0)
  (Ability|EndAbility))