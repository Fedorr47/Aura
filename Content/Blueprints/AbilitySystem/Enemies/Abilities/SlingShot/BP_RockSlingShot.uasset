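; BP_RockSlingShot is a rock actor for the enemy slingshot ability, with logic to spin its mesh.
; BeginPlay sets three rotation rates from random ranges, all bounded at zero, so the rock does not rotate as written.
; Tick scales the rates by delta time and adds them as local rotation to RockMesh, with rate names mismatched to the axes they drive.
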(event EventBeginPlay
  (bind _returnvalue (Math|Random|RandomFloatinRange 0.0 0.0))
  (Variables|Default|SetYawRoationRate _returnvalue)
  (Variables|Default|SetRollRoationRate _returnvalue)
  (Variables|Default|SetPitchRoationRate _returnvalue))

(event Collision|EventActorBeginOverlap
  (params (OtherActor :type Actor%20Object%20Reference)))

(event EventTick
  (params (DeltaSeconds :type Float%20%28single-precision%29))
  (Variables|Default|SetDelta%20Seconds DeltaSeconds)
  (Transformation|AddLocalRotation (Variables|Default|GetRockMesh) (Math|Rotator|MakeRotator (* (Variables|Default|GetDelta%20Seconds) (Variables|Default|GetYawRoationRate)) (* (Variables|Default|GetRollRoationRate) (Variables|Default|GetDelta%20Seconds)) (* (Variables|Default|GetPitchRoationRate) (Variables|Default|GetDelta%20Seconds))) false false))

(fn ConstructionScript)