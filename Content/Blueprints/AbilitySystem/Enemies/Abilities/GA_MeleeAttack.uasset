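; Enemy melee attack Gameplay Ability that turns the avatar toward its combat target and plays a randomly chosen attack montage from the CombatInterface.
; A gameplay event matching the montage's tag triggers a small sphere query at that tag's combat socket location, damaging each live non-friend actor found.
; The ability ends after that hit check or when the montage completes, is interrupted or is cancelled.
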(event Ability|EventActivateAbility
  (bind _output_get (Variables|Default|SetAbilityOwnerActor (Ability|GetAvatarActorfromActorInfo)))
  (bind _returnvalue (Class|EnemyInterface|GetCombatTarget(Message) _output_get))
  (bind _output_get_2 (Variables|Default|SetCombatTarget _returnvalue))
  (Utilities|IsValid _output_get_2
    (:Is%20Valid
      (bind _ascombat_interface (Utilities|Casting|CastToCombatInterface (Variables|Default|GetAbilityOwnerActor)))
      (Class|CombatInterface|SetFacingWrapping _ascombat_interface (Transformation|GetActorLocation (Variables|Default|GetCombatTarget)))
      (bind _returnvalue_2 (Class|CombatInterface|GetAttackMontage _ascombat_interface))
      (if (> (Utilities|Array|Length _returnvalue_2) 0)
        (bind _output_get_3 (Variables|Default|SetTaggedMontage (Utilities|Array|Get(acopy) _returnvalue_2 (Math|Random|RandomIntegerinRange 0 (- (Utilities|Array|Length _returnvalue_2) 1)))))
        (|PlayMontageandWaitProxy "None" (.Montage (Utilities|Struct|BreakTaggedMontage _output_get_3)) 1.0 "None" false 1.0 0.0 false
          (:then
            (Ability|Tasks|WaitGameplayEvent (.MontageTag (Utilities|Struct|BreakTaggedMontage _output_get_3)) 0
              (:EventReceived
                (bind _returnvalue_3 (Class|CombatInterface|GetCombatSocketLocation(Message) (Variables|Default|GetAbilityOwnerActor) (.MontageTag (Utilities|Struct|BreakTaggedMontage _output_get_3))))
                (bind _outoverlappingactors (Class|AuraAbilitySystemLibrary|GetLivePlayerswithRadius (Variables|Default|GetAbilityOwnerActor) (Utilities|Array|MakeArray (Variables|Default|GetAbilityOwnerActor)) 45.0 _returnvalue_3))
                (for _array_element _outoverlappingactors
                  (if (Class|AuraAbilitySystemLibrary|IsNotFriend (Variables|Default|GetAbilityOwnerActor) _array_element)
                    (Class|AuraDamageGameplayAbility|DoDamage _array_element)))
                (Ability|EndAbility))))
          (:OnCompleted
            (Ability|EndAbility :!label _label))
          (:OnInterrupted
            (goto _label))
          (:OnCancelled
            (goto _label)))))))

(event Ability|EventOnEndAbility
  (params (bWasCancelled :type Boolean)))